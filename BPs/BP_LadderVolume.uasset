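; BP_LadderVolume is a ladder trigger volume that automatically moves the player character upward while it overlaps.
; BeginPlay caches the player's BP_Character and creates a paused, looping Climb timer.
; Overlap begin switches movement to Flying and unpauses the timer, which repeatedly adds upward movement input; overlap end restores Walking and pauses it.
; Climb's branch is hardwired true, so it reads no player input and never takes its exit path.
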(event `self.ReceiveBeginPlay`
  (bind _asbp_character (cast `/Game/BPs/BP_Character` (`GameplayStatics.GetPlayerCharacter` 0)))
  (set `self.As BP Character` _asbp_character)
  (`KismetSystemLibrary.K2_SetTimer` null "Climb" 0.03 true)
  (`KismetSystemLibrary.K2_PauseTimer` null "Climb"))

(event `self.Volume.OnComponentBeginOverlap`
  (params (OverlappedComponent :type "PrimitiveComponent Object Reference") (OtherActor :type "Actor Object Reference") (OtherComp :type "PrimitiveComponent Object Reference") (OtherBodyIndex :type Integer) (bFromSweep :type Boolean) (SweepResult :type "HitResult Structure (by ref)"))
  (bind _as_bp_character (`self.As BP Character`))
  (if (== OtherActor _as_bp_character)
    (set `self.Climbing` true)
    (`CharacterMovementComponent.SetMovementMode` (`Character.CharacterMovement` _as_bp_character) "MOVE_Flying" 0)
    (`KismetSystemLibrary.K2_UnPauseTimer` null "Climb")))

(event `self.Volume.OnComponentEndOverlap`
  (params (OverlappedComponent :type "PrimitiveComponent Object Reference") (OtherActor :type "Actor Object Reference") (OtherComp :type "PrimitiveComponent Object Reference") (OtherBodyIndex :type Integer))
  (bind _as_bp_character (`self.As BP Character`))
  (if (== OtherActor _as_bp_character)
    (set `self.Climbing` false :!label _label)
    (`CharacterMovementComponent.SetMovementMode` (`Character.CharacterMovement` _as_bp_character) "MOVE_Walking" 0)
    (`KismetSystemLibrary.K2_PauseTimer` null "Climb")))

(event `Climb`
  (if true
    (`Pawn.AddMovementInput` (`self.As BP Character`) (0.0 0.0 1.0) 1.0 false)
    (else
      (goto _label))))

(fn `UserConstructionScript`)