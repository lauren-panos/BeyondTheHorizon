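; Player character Blueprint with Enhanced Input movement and look, double jump, a pause menu, physics-object grabbing and projectile shooting.
; Holding E line-traces from the mesh and grabs the hit component with a PhysicsHandle, repositioned each Tick.
; Firing spawns BP_Projectile at the muzzle, gated by CheckReady on magazine ammo and a delayed reload from reserve.
; Landing restores the double jump; pausing toggles WBP_Pause, cursor and input mode.
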(event `EnhancedInput|/Game/BPs/IO/IA_Pause`
  (params (ActionValue :type Boolean) (ElapsedSeconds :type "Float (double-precision)") (TriggeredSeconds :type "Float (double-precision)") (InputAction :type "InputAction Object Reference" :default "/Game/BPs/IO/IA_Pause.IA_Pause"))
  (bind _returnvalue (`GameplayStatics.GetPlayerController` 0))
  ;[1 1 1] Pause Menu
  (:`Started`
    (if (not (`self.IsPauseOpen`))
      (set `self.IsPauseOpen` true)
      (bind _returnvalue_2 (`|CreateWidget` "/Game/BPs/UI/WBP_Pause.WBP_Pause_C" _returnvalue))
      (bind _output_get (set `self.Pause Menu Widget` _returnvalue_2))
      (`UserWidget.AddToViewport` _output_get 0)
      (`WidgetBlueprintLibrary.SetInputMode_GameAndUIEx` _returnvalue (`self.Pause Menu Widget`))
      (set `PlayerController.bShowMouseCursor` true (`GameplayStatics.GetPlayerController` 0))
      (`GameplayStatics.SetGamePaused` true)
      (else
        (set `self.IsPauseOpen` false)
        (`Widget.RemoveFromParent` (`self.Pause Menu Widget`))
        (`GameplayStatics.SetGamePaused` false)
        (`WidgetBlueprintLibrary.SetInputMode_GameOnly` _returnvalue)
        (set `PlayerController.bShowMouseCursor` false (`GameplayStatics.GetPlayerController` 0))))))

(event `self.ReceiveBeginPlay`
  ;[1 1 1] Establish IMC
  (`EnhancedInputSubsystemInterface.AddMappingContext` (pcsubsystem `EnhancedInputLocalPlayerSubsystem` (`GameplayStatics.GetPlayerController` 0)) "/Game/BPs/IO/IMC_BaseCharacter.IMC_BaseCharacter" 0 (struct)))

(event `EnhancedInput|/Game/BPs/IO/IA_Locomotion2`
  (params (ActionValue :type "Float (double-precision)") (ElapsedSeconds :type "Float (double-precision)") (TriggeredSeconds :type "Float (double-precision)") (InputAction :type "InputAction Object Reference" :default "/Game/BPs/IO/IA_Locomotion2.IA_Locomotion2"))
  ;[1 1 1] Core Movement
  (:`Triggered`
    (`self.AddMovementInput` (`self.GetActorForwardVector`) ActionValue)))

(event `EnhancedInput|/Game/BPs/IO/IA_Strafe2`
  (params (ActionValue :type "Float (double-precision)") (ElapsedSeconds :type "Float (double-precision)") (TriggeredSeconds :type "Float (double-precision)") (InputAction :type "InputAction Object Reference" :default "/Game/BPs/IO/IA_Strafe2.IA_Strafe2"))
  ;[1 1 1] Core Movement
  (:`Triggered`
    (`self.AddMovementInput` (`self.GetActorRightVector`) ActionValue)))

(event `Key|E`
  (params (Key :type "Key Structure"))
  (bind _mesh (`self.Mesh`))
  (bind _returnvalue (`SceneComponent.K2_GetComponentLocation` _mesh))
  ;[1 1 1] Grabbing System
  (:`Pressed`
    (bind (_outhit _returnvalue_2) (`KismetSystemLibrary.LineTraceSingle` _returnvalue (+ _returnvalue (* (`KismetMathLibrary.GetForwardVector` (`SceneComponent.K2_GetComponentRotation` _mesh)) 500.0)) "TraceTypeQuery1"))
    (if _returnvalue_2
      (bind (_bblockinghit _binitialoverlap _time _distance _location _impactpoint _normal _impactnormal _physmat _hitactor _hitcomponent) (`GameplayStatics.BreakHitResult` _outhit))
      (`PhysicsHandleComponent.GrabComponentAtLocationWithRotation` :`self` (`self.PhysicsHandle`) :`Component` _hitcomponent :`Location` (`SceneComponent.K2_GetComponentLocation` _hitcomponent))
      (set `self.isGrabbingObject` true)))
  (:`Released`
    (if (`self.isGrabbingObject`)
      (`PhysicsHandleComponent.ReleaseComponent` (`self.PhysicsHandle`))
      (set `self.isGrabbingObject` false))))

(event `EnhancedInput|/Game/BPs/IO/Ia_LookV2`
  (params (ActionValue :type "Float (double-precision)") (ElapsedSeconds :type "Float (double-precision)") (TriggeredSeconds :type "Float (double-precision)") (InputAction :type "InputAction Object Reference" :default "/Game/BPs/IO/Ia_LookV2.Ia_LookV2"))
  ;[1 1 1] Core Movement
  (:`Triggered`
    (`self.AddControllerPitchInput` ActionValue)))

(event `EnhancedInput|/Game/BPs/IO/IA_LookH2`
  (params (ActionValue :type "Float (double-precision)") (ElapsedSeconds :type "Float (double-precision)") (TriggeredSeconds :type "Float (double-precision)") (InputAction :type "InputAction Object Reference" :default "/Game/BPs/IO/IA_LookH2.IA_LookH2"))
  ;[1 1 1] Core Movement
  (:`Triggered`
    (`self.AddControllerYawInput` ActionValue)))

(event `self.K2_OnMovementModeChanged`
  (params (PrevMovementMode :type "EMovementMode Enum" :default "MOVE_None") (NewMovementMode :type "EMovementMode Enum" :default "MOVE_None") (PrevCustomMode :type Byte) (NewCustomMode :type Byte))
  (switch `EMovementMode` PrevMovementMode
    (:`MOVE_Walking`
      (`/Engine/EditorBlueprintResources/StandardMacros.DoOnce` false :!via `Reset`
        (:`Completed`
          (`self.Adjust Jump` (`CharacterMovementComponent.JumpZVelocity` (`self.CharacterMovement`)))
          (`self.LaunchCharacter` (0.0 0.0 500.0) false true))))))

(event `EnhancedInput|/Game/BPs/IO/IA_Jump`
  (params (ActionValue :type Boolean) (ElapsedSeconds :type "Float (double-precision)") (TriggeredSeconds :type "Float (double-precision)") (InputAction :type "InputAction Object Reference" :default "/Game/BPs/IO/IA_Jump.IA_Jump"))
  ;[1 1 1] Double jump
  (:`Started`
    (`self.Jump`)
    (if (and (`self.doubleJump`) (`NavMovementComponent.IsFalling` (`self.CharacterMovement`)))
      (set `self.doubleJump` false)
      (`self.LaunchCharacter` (`KismetMathLibrary.MakeVector` 0.0 0.0 (`CharacterMovementComponent.JumpZVelocity` (`self.CharacterMovement`))) false true)))
  (:`Completed`
    (`self.StopJumping`)))

(event `self.ReceiveTick`
  (params (DeltaSeconds :type "Float (single-precision)"))
  (bind _mesh (`self.Mesh`))
  ;[1 1 1] Object Picked Up Loop
  (if (`self.isGrabbingObject`)
    (`PhysicsHandleComponent.SetTargetLocation` (`self.PhysicsHandle`) (+ (`SceneComponent.K2_GetComponentLocation` _mesh) (* (`KismetMathLibrary.GetForwardVector` (`SceneComponent.K2_GetComponentRotation` _mesh)) 500.0)))))

(event `self.OnLanded`
  (params (Hit :type "HitResult Structure (by ref)"))
  ;[1 1 1] Double jump
  (set `self.doubleJump` true))

(event `EnhancedInput|/Game/BPs/IO/IA_Primary`
  (params (ActionValue :type "Float (double-precision)") (ElapsedSeconds :type "Float (double-precision)") (TriggeredSeconds :type "Float (double-precision)") (InputAction :type "InputAction Object Reference" :default "/Game/BPs/IO/IA_Primary.IA_Primary"))
  ;[1 1 1] Shooting/Reload
  (:`Started`
    (if (`self.CheckReady`)
      (`/Engine/EditorBlueprintResources/StandardMacros.DecrementInt` (`self.magAmmo`)
        (:`  `
          (`|SpawnActorFromClass` "/Game/BPs/BP_Projectile.BP_Projectile_C" (`SceneComponent.K2_GetComponentToWorld` (`self.Muzzle`)) "Undefined" "MultiplyWithRoot" null self))))))

(event `EnhancedInput|/Game/BPs/IO/IA_Reload`
  (params (ActionValue :type "Float (double-precision)") (ElapsedSeconds :type "Float (double-precision)") (TriggeredSeconds :type "Float (double-precision)") (InputAction :type "InputAction Object Reference" :default "/Game/BPs/IO/IA_Reload.IA_Reload"))
  ;[1 1 1] Shooting/Reload
  (:`Triggered`
    (if (and (< (`self.magAmmo`) (`self.magMax`)) (> (`self.reserveAmmo`) 0))
      (set `self.Reloading` true)
      (`KismetSystemLibrary.Delay` 1.25)
      (if (> (`self.reserveAmmo`) (`self.magMax`))
        (bind _output_get (set `self.magAmmo` (`self.magMax`)))
        (set `self.reserveAmmo` (- (`self.reserveAmmo`) _output_get))
        (else
          (set `self.magAmmo` (`self.reserveAmmo`))
          (set `self.reserveAmmo` 0)))
      (set `self.Reloading` false))))

(fn `Adjust Jump`
  (params (Effect :type "Float (double-precision)"))
  (`parent.Adjust Jump` Effect)
  (set `CharacterMovementComponent.JumpZVelocity` Effect (`self.CharacterMovement`)))

(fn `CheckReady`
  (returns (`is Fire Ready` :type Boolean))
  (return (not (or (`self.Reloading`) (<= (`self.magAmmo`) 0)))))

(fn `ResetJumpHeight`
  (set `CharacterMovementComponent.JumpZVelocity` 500.0 (`self.CharacterMovement`))
  (set `self.Bounding` false))

(fn `UserConstructionScript`)